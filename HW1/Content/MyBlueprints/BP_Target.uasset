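; BP_Target is a moving shootable target with a health bar that counts toward the player's goal when destroyed.
; A Timeline started on BeginPlay lerps it between start and end positions and repeatedly assigns itself as the health bar widget's owner.
; First-person projectile hits subtract fixed damage; at zero health it destroys itself, increments the character's TargetsHit and calls CheckGoal.
; Tick rotates the widget to face the player.
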(event `self.ReceiveHit`
  (params (MyComp :type "PrimitiveComponent Object Reference") (Other :type "Actor Object Reference") (OtherComp :type "PrimitiveComponent Object Reference") (bSelfMoved :type Boolean) (HitLocation :type "Vector Structure") (HitNormal :type "Vector Structure") (NormalImpulse :type "Vector Structure") (Hit :type "HitResult Structure (by ref)"))
  (cast `/Game/FirstPerson/Blueprints/BP_FirstPersonProjectile` Other)
  (bind _asbp_first_person_character (cast `/Game/FirstPerson/Blueprints/BP_FirstPersonCharacter` (`GameplayStatics.GetPlayerCharacter` 0)))
  (bind _output_get (set `self.Health` (- (`self.Health`) 20.0)))
  (`KismetSystemLibrary.PrintString` (`KismetStringLibrary.Conv_DoubleToString` _output_get))
  (if (<= _output_get 0.0)
    (`self.K2_DestroyActor`)
    (`/Engine/EditorBlueprintResources/StandardMacros.IncrementInt` (`/Game/FirstPerson/Blueprints/BP_FirstPersonCharacter.TargetsHit` _asbp_first_person_character)
      (:`  `
        (`/Game/FirstPerson/Blueprints/BP_FirstPersonCharacter.CheckGoal` _asbp_first_person_character)))))

(event `self.ReceiveBeginPlay`
  (bind (_direction _alpha) (`Timeline|MovementTimeline` :!via `PlayFromStart`)
    (:`Update`
      (`self.K2_SetActorLocation` (`KismetMathLibrary.VLerp` (`self.StartPosition`) (`self.EndPosition`) _alpha))
      (bind _astarget_health_bar (cast `/Game/FirstPerson/Blueprints/Target_HealthBar` (`WidgetComponent.GetUserWidgetObject` (`self.Widget`))))
      (set `/Game/FirstPerson/Blueprints/Target_HealthBar.OwningActor` self _astarget_health_bar))))

(event `self.ReceiveTick`
  (params (DeltaSeconds :type "Float (single-precision)"))
  (`SceneComponent.K2_SetWorldRotation` (`self.Widget`) (`KismetMathLibrary.FindLookAtRotation` (`self.K2_GetActorLocation` self) (`self.K2_GetActorLocation` (`GameplayStatics.GetPlayerCharacter` 0))) false false))

(fn `UserConstructionScript`)